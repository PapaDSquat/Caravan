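; Base actor for caravan base camp buildings that the player constructs through interaction, then uses for crafting menus.
; Each Construct interaction advances building by a fixed step; progress events drive a camera-facing percent text, and state changes swap unconstructed and built meshes and collision.
; Interaction choices rebuild dynamically: Construct until built, then a Craft submenu listing inventory items with descriptions and required materials.
; Only Construct is handled here; CraftItem choices have no handler.
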(event Custom|OnInteract
  (params (InteractingPawn :type Pawn%20Object%20Reference) (InteractableComponent :type Interactable%20Component%20Object%20Reference) (Choice :type Interaction%20Choice%20Structure%20%28by%20ref%29))
  (switch name (.InteractionID (Utilities|Struct|BreakInteractionChoice Choice))
    (:Construct
      (Class|CampBuildingActor|ConstructBuilding 0.05))))

(event Custom|OnInteractionRebuildChoices
  (params (InteractingPawn :type Pawn%20Object%20Reference) (InteractableComponent :type Interactable%20Component%20Object%20Reference))
  (Class|InteractableComponent|SetInteractionChoices InteractableComponent (Interaction|BuildInteractionChoices)))

(event EventBeginPlay
  (bind _interactablecomponent (Variables|Default|GetInteractableComponent))
  (Utilities|FlowControl|Sequence
    (:then_0
      (Rendering|SetVisibility (Variables|Default|GetConstructionPercentText) false false))
    (:then_1
      (EventDispatchers|BindEventtoOnInteract _interactablecomponent (delegate Custom|OnInteract))
      (EventDispatchers|BindEventtoOnRebuildInteractionChoices _interactablecomponent (delegate Custom|OnInteractionRebuildChoices)))))

(event EventTick
  (params (DeltaSeconds :type Float%20%28single-precision%29))
  (Transformation|SetWorldRotation (Variables|Default|GetConstructionPercentText) (Math|Rotator|MakeRotfromX (* (Math|Vector|GetForwardVector (Camera|GetCameraRotation (Game|GetPlayerCameraManager 0))) "-1.000000,1.000000,-1.000000")) false false))

(event EventOnBuildingStateChange
  (params (OldState :type ECampBuildingState%20Enum :default "Deconstructed") (NewState :type ECampBuildingState%20Enum :default "Deconstructed"))
  (bind _unconstructedmesh (Variables|Default|GetUnconstructedMesh))
  (bind _buildingmesh (Variables|Default|GetBuildingMesh))
  (bind _buildingmesh_2 (Variables|Default|GetBuildingMesh))
  (switch Utilities|FlowControl|Switch|SwitchonECampBuildingState NewState
    (:Deconstructed
      (Rendering|SetVisibility _unconstructedmesh true true)
      (Rendering|SetVisibility _buildingmesh false true)
      (Collision|SetCollisionEnabled _buildingmesh_2 "NoCollision"))
    (:Constructed
      (Rendering|SetVisibility _unconstructedmesh false true)
      (Rendering|SetVisibility _buildingmesh true true)
      (Collision|SetCollisionEnabled _buildingmesh_2 "QueryAndPhysics"))))

(event EventOnBuildingConstructProgress
  (params (CurrentPercent :type Float%20%28single-precision%29))
  (bind _constructionpercenttext (Variables|Default|GetConstructionPercentText))
  (Rendering|SetVisibility _constructionpercenttext true false)
  (Rendering|Components|TextRender|SetText _constructionpercenttext (Utilities|Text|ToText(Float) (* CurrentPercent 1e+02) "HalfToEven" false true 2 3 0 0)))

(event EventOnBuildingConstructed
  (Rendering|SetVisibility (Variables|Default|GetConstructionPercentText) false false))

(fn ConstructionScript)

(fn BuildInteractionChoices
  (Utilities|FlowControl|Sequence
    (:then_0
      (if (Class|CampBuildingActor|IsConstructed)
        (switch name (Class|InteractableComponent|GetCurrentInteractionSubChoice (Variables|Default|GetInteractableComponent))
          (:Default
            (LocalVariables|SetOutChoices (Utilities|Array|MakeArray (Utilities|Struct|MakeInteractionChoice "Craft" "Craft" "" "None" "Craft"))))
          (:Craft
            (for _array_element (Class|InventoryComponent|GetItemStacks (Variables|Default|GetInventoryComponent))
              (bind (_isvalid _returnvalue) (Interaction|BuildCraftItemInteractionChoice _array_element))
              (if _isvalid
                (Utilities|Array|Add (LocalVariables|GetOutChoices) _returnvalue)))))
        (else
          (Utilities|Array|Add (LocalVariables|GetOutChoices) (Utilities|Struct|MakeInteractionChoice "Construct" "Construct")))))
    (:then_1
      (return (LocalVariables|GetOutChoices)))))

(fn BuildCraftItemInteractionChoice
  (params (ItemStack :type Item%20Stack%20Structure))
  (bind (_itemhandle _count _binfinite) (Utilities|Struct|BreakItemStack ItemStack))
  (bind (_outitemdef _returnvalue) (Class|InventoryFunctionLibrary|GetItemDefinition _itemhandle))
  (bind (_itemid _resourcetype _displayname _description _displaypriority _staticmesh _meshscale _uiicon _materialstocraft) (Utilities|Struct|BreakInventoryItemDataRow _outitemdef))
  (bind _result (Utilities|Text|FormatText "{ItemName}" _displayname))
  (if _returnvalue
    (for _array_element _materialstocraft
      (if (.ReturnValue (Class|InventoryFunctionLibrary|GetItemDefinition (.ItemHandle (Utilities|Struct|BreakItemStack _array_element))))
        (LocalVariables|SetCraftMaterialsStr (Utilities|String|Append (LocalVariables|GetCraftMaterialsStr) (Utilities|String|ToString(Text) (Utilities|Text|FormatText "{ItemName} ({ItemCount})      " (.DisplayName (Utilities|Struct|BreakInventoryItemDataRow (.OutItemDef (Class|InventoryFunctionLibrary|GetItemDefinition (.ItemHandle (Utilities|Struct|BreakItemStack _array_element)))))) (.Count (Utilities|Struct|BreakItemStack _array_element))))))))
    (return true (Utilities|Struct|MakeInteractionChoice "CraftItem" (select _binfinite _result _result) (select (Utilities|Array|IsEmpty (LocalVariables|GetCraftMaterialsStr)) (Utilities|Text|FormatText "{ItemDesc}" _description) (Utilities|Text|FormatText "{ItemDesc}\\n{CraftMaterials}" _description (LocalVariables|GetCraftMaterialsStr))) "None" ""))
    (else
      (return false ""))))