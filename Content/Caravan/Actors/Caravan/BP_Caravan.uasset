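; BP_Caravan is the caravan actor, with a back door that switches between open and closed states.
; Its NotifyonToggleOpen event snaps the door to a fixed rotation and position for each state and shows or hides both ramps and the base board.
; The change is instant, with rotation set in world space and location in relative space, so the pose assumes an unrotated caravan.
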(event EventBeginPlay)

(event Collision|EventActorBeginOverlap
  (params (OtherActor :type Actor%20Object%20Reference)))

(event EventTick
  (params (DeltaSeconds :type Float%20%28single-precision%29)))

(event EventNotifyonToggleOpen
  (params (Open :type Boolean))
  (bind _caravanrampleft (Variables|Default|GetCaravanRampLeft))
  (bind _caravanrampright (Variables|Default|GetCaravanRampRight))
  (bind _caravanbaseboard (Variables|Default|GetCaravanBaseBoard))
  (bind _caravanbackdoor (Variables|Default|GetCaravanBackDoor))
  (bind _array (Utilities|Array|MakeArray _caravanrampleft _caravanrampright _caravanbaseboard))
  ;[1 1 1] Toggle Open/Close
  (if Open
    (Transformation|SetWorldRotation _caravanbackdoor "90.000000, 0, 0" false false)
    (Transformation|SetRelativeLocation _caravanbackdoor "-320.000000,0.000000,0.000000" false true)
    (Rendering|SetVisibility _array true false)
    (else
      (Transformation|SetWorldRotation _caravanbackdoor "0, 0, 0" false false)
      (Transformation|SetRelativeLocation _caravanbackdoor "-195.000000, 0,130.000000" false true)
      (Rendering|SetVisibility _array false false))))

(fn ConstructionScript)