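; Caravan building platform actor that shows a world-space craft UI widget while it has interaction focus.
; The widget starts hidden, appears on first focus and hides again on unfocus; the select event is empty.
; Each tick, it yaws the widget toward the player character, building the rotation from the flattened UISocket-to-player direction and a downward up axis.
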(event EventBeginPlay
  (Rendering|SetVisibility (Variables|Default|GetUICraftWidget) false false))

(event EventNotifyonInteractUnFocus
  (Rendering|SetVisibility (Variables|Default|GetUICraftWidget) false false))

(event EventNotifyonInteractSelect)

(event EventTick
  (params (DeltaSeconds :type Float%20%28single-precision%29))
  (bind _returnvalue (Game|GetPlayerCharacter 0))
  (bind _returnvalue_2 (Math|Vector|MakeVector 0.0 0.0 -1.0))
  (bind _staticmeshcomponent (Variables|Default|GetStaticMeshComponent))
  (bind _returnvalue_3 (Transformation|GetSocketLocation _staticmeshcomponent "UISocket"))
  (bind _returnvalue_4 (Transformation|GetActorLocation _returnvalue))
  (bind _returnvalue_5 (Math|Vector|GetUnitDirection(Vector) _returnvalue_3 _returnvalue_4))
  (bind (_x _y) (Math|Vector|BreakVector _returnvalue_5))
  (bind _returnvalue_6 (Math|Vector|MakeVector _x _y 0.0))
  (Utilities|IsValid _returnvalue
    (:Is%20Valid
      (Transformation|SetWorldRotation (Variables|Default|GetUICraftWidget) (Math|Rotator|MakeRotationfromAxes _returnvalue_6 (Math|Vector|CrossProduct _returnvalue_6 _returnvalue_2) _returnvalue_2) false false))))

(event EventNotifyonInteractFirstFocus
  (Rendering|SetVisibility (Variables|Default|GetUICraftWidget) true false))

(fn ConstructionScript)